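; GA_SystemReset is a gameplay ability that temporarily marks an enemy as uploading, apparently for a System Reset quickhack.
; On activation it starts a one-shot wait for the QH.SystemReset event, then immediately commits cost and cooldown and starts the startup delay.
; The event's payload target receives the QH.Uploading tag, which is removed when the delay finishes.
; The ability only ends itself when the BP_EnemyBase cast fails; no reset effect is implemented here.
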(event Ability|EventActivateAbility
  (bind (_asynctaskproxy _payload) (Ability|Tasks|WaitGameplayEvent "(TagName=\"QH.SystemReset\")" 0 true)
    (:then
      (Variables|Default|SetGameplayAsyncTask _asynctaskproxy)
      (Ability|CommitAbilityCost false)
      (Ability|CommitAbilityCooldown false)
      (Ability|Tasks|WaitDelay (Variables|Default|GetDefaultStartupDelay)
        (:OnFinish
          (bind _asbp_enemy_base (Utilities|Casting|CastToBP_EnemyBase (Variables|Default|GetTarget))
            (:then
              (Class|CharacterBase|RemoveGameplayTag _asbp_enemy_base (GameplayTags|MakeLiteralGameplayTag "(TagName=\"QH.Uploading\")")))
            (:CastFailed
              (Ability|EndAbility))))))
    (:EventReceived
      (bind _output_get (Variables|Default|SetPayload _payload))
      (bind _output_get_2 (Variables|Default|SetTarget (.Target (Utilities|Struct|BreakGameplayEventData _output_get))))
      (bind _asbp_enemy_base_2 (Utilities|Casting|CastToBP_EnemyBase _output_get_2)
        (:then
          (Class|CharacterBase|AddGameplayTag _asbp_enemy_base_2 (GameplayTags|MakeLiteralGameplayTag "(TagName=\"QH.Uploading\")")))
        (:CastFailed
          (Ability|EndAbility))))))

(event Ability|EventOnEndAbility
  (params (bWasCancelled :type Boolean)))