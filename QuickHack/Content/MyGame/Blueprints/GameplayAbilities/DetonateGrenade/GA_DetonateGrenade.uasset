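; GA_DetonateGrenade is a gameplay ability that detonates a grenade on a targeted enemy, damaging enemies around it.
; On activation it listens for the QH.DetonateGrenade event, which supplies the target and tags it QH.Uploading, while cost, cooldown and startup delay run without waiting for that event.
; After the delay it clears the tag, sphere-traces at the target with persistent debug drawing, and applies GE_DetonateGrenade_Damage to enemies hit.
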(event Ability|EventActivateAbility
  (bind (_asynctaskproxy _payload) (Ability|Tasks|WaitGameplayEvent "(TagName=\"QH.DetonateGrenade\")" 0 true)
    (:then
      (Variables|Default|SetGameplayAsyncTask _asynctaskproxy)
      (Ability|CommitAbilityCost false)
      (Ability|CommitAbilityCooldown false)
      (Ability|Tasks|WaitDelay (Variables|Default|GetDefaultStartupDelay)
        (:OnFinish
          (bind _asbp_enemy_base (Utilities|Casting|CastToBP_EnemyBase (Variables|Default|GetTarget))
            (:then
              (Class|CharacterBase|RemoveGameplayTag _asbp_enemy_base (GameplayTags|MakeLiteralGameplayTag "(TagName=\"QH.Uploading\")"))
              (bind _outhits (Collision|MultiSphereTraceByChannel (Transformation|GetActorLocation (Variables|Default|GetTarget)) (Transformation|GetActorLocation (Variables|Default|GetTarget)) (Variables|Default|GetRadius) "TraceTypeQuery3" false (Utilities|Array|MakeArray (.AsBP%20Player%20Character (Utilities|Casting|CastToBP_PlayerCharacter (Ability|GetCurrentSourceObject)))) "Persistent"))
              (for _array_element _outhits
                (bind _asbp_enemy_base_2 (Utilities|Casting|CastToBP_EnemyBase (.HitActor (Collision|BreakHitResult _array_element))))
                (GameplayEffects|ApplyGameplayEffectToSelf :self (Variables|/Script/QuickHack.CharacterBase|GetAbilitySystemComponent _asbp_enemy_base_2) :GameplayEffectClass "/Game/MyGame/Blueprints/GameplayAbilities/DetonateGrenade/GE_DetonateGrenade_Damage.GE_DetonateGrenade_Damage_C"))
              (Ability|EndAbility))
            (:CastFailed
              (Ability|EndAbility))))))
    (:EventReceived
      (bind _output_get (Variables|Default|SetPayload _payload))
      (bind _output_get_2 (Variables|Default|SetTarget (.Target (Utilities|Struct|BreakGameplayEventData _output_get))))
      (bind _asbp_enemy_base_3 (Utilities|Casting|CastToBP_EnemyBase _output_get_2)
        (:then
          (Class|CharacterBase|AddGameplayTag _asbp_enemy_base_3 (GameplayTags|MakeLiteralGameplayTag "(TagName=\"QH.Uploading\")")))
        (:CastFailed
          (Ability|EndAbility))))))

(event Ability|EventOnEndAbility
  (params (bWasCancelled :type Boolean)))