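; First-person player character Blueprint that runs a quickhack system on enemies and feeds health and cyberdeck RAM to the HUD widgets.
; While tracing is enabled, a per-tick camera trace picks the BP_EnemyBase target, with DoOnce gates throttling target notifications.
; List inputs cycle the hack panels; confirm activates the selected GAS ability on targets not already uploading, sends a gameplay event, and starts upload and cooldown.
; BeginPlay also contains a leftover debug print loop.
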(event Custom|PerformQuickHack
  (params (EventTag :type Gameplay%20Tag%20Structure) (QuickHackInfo :type Gameplay%20Quick%20Hack%20Ability%20Info%20Structure) (InAbilityToActivate :type Gameplay%20Ability%20Class%20Reference))
  (if (Math|Boolean|ANDBoolean (Utilities|IsValid (Variables|Default|GetQuickHackTarget)) (Variables|Default|GetbTargetAquired) (not (Class|CharacterBase|HasGameplayTag (Variables|Default|GetQuickHackTarget) (GameplayTags|MakeLiteralGameplayTag "(TagName=\"QH.Uploading\")"))))
    (bind _returnvalue (Abilities|TryActivateAbilitybyClass (Variables|Default|GetAbilitySystemComponent) InAbilityToActivate true))
    (if _returnvalue
      (Ability|SendGameplayEventtoActor self EventTag (Utilities|Struct|MakeGameplayEventData "" self (Variables|Default|GetQuickHackTarget) 0 0 "()" "(GameplayTags=)" "(GameplayTags=((TagName=\"QH.Uploading\")))"))
      (Default|StartQuickHackUpload (Variables|Default|GetQuickHackTarget) QuickHackInfo)
      (bind _aswbp_quick_hack_hud (Utilities|Casting|CastToWBP_QuickHackHUD (Variables|Default|GetQuickHackWidget)))
      (Default|DoUIAbilityCooldown (Utilities|Array|Get(acopy) (Variables|/Game/MyGame/Blueprints/UI/WBP_QuickHackHUD.WBP_QuickHackHUD_C|GetQuickHackPanels _aswbp_quick_hack_hud) (Variables|Default|GetCurrentSelectedPanelIndex))))))

(event Custom|DoLineTrace
  (bind _firstpersoncameracomponent (Variables|Default|GetFirstPersonCameraComponent))
  (bind _returnvalue (Transformation|GetWorldLocation _firstpersoncameracomponent))
  (bind _outhit (Collision|LineTraceByChannel _returnvalue (+ _returnvalue (* (Math|Vector|GetForwardVector (Transformation|GetWorldRotation _firstpersoncameracomponent)) 5e+03)) "TraceTypeQuery1" false (Utilities|Array|MakeArray self) "None"))
  ;[1 1 1] Sets The target that will get effected by the ability
  (bind _asbp_enemy_base (Utilities|Casting|CastToBP_EnemyBase (.HitActor (Collision|BreakHitResult _outhit)))
    (:then
      (Variables|Default|SetQuickHackTarget _asbp_enemy_base)
      (bind _output_get (Variables|Default|SetbTargetAquired true))
      (Utilities|FlowControl|Sequence
        (:then_0
          (Utilities|FlowControl|DoOnce false :!label _label
            (:Completed
              (Default|CallOnQuickHackTargetAquired _output_get))))
        (:then_1
          (goto _label_2 Reset))))
    (:CastFailed
      (Variables|Default|SetQuickHackTarget 0)
      (bind _output_get_2 (Variables|Default|SetbTargetAquired false))
      (Utilities|FlowControl|Sequence
        (:then_0
          (Utilities|FlowControl|DoOnce false :!label _label_2
            (:Completed
              (Default|CallOnQuickHackTargetAquired _output_get_2))))
        (:then_1
          (goto _label Reset))))))

(event EventAddAbilitytoUI
  (params (AbilityInfo :type Gameplay%20Quick%20Hack%20Ability%20Info%20Structure))
  (bind _aswbp_quick_hack_hud (Utilities|Casting|CastToWBP_QuickHackHUD (Variables|Default|GetQuickHackWidget))
    (:then
      (Utilities|IsValid (Utilities|Array|Get(acopy) (Variables|/Game/MyGame/Blueprints/UI/WBP_QuickHackHUD.WBP_QuickHackHUD_C|GetQuickHackPanels _aswbp_quick_hack_hud) (Variables|Default|GetQuickHackPanelCount))
        (:Is%20Valid
          (Default|UpdateQuickHackValues (Utilities|Array|Get(acopy) (Variables|/Game/MyGame/Blueprints/UI/WBP_QuickHackHUD.WBP_QuickHackHUD_C|GetQuickHackPanels _aswbp_quick_hack_hud) (Variables|Default|GetQuickHackPanelCount)) AbilityInfo)
          (Variables|Default|SetQuickHackPanelCount (+ (Variables|Default|GetQuickHackPanelCount) 1)))
        (:Is%20Not%20Valid
          (Development|PrintString "Target panel isn't valid"))))
    (:CastFailed
      (Development|PrintString "quickhack WBP cxast failed"))))

(event EventOnHealthChanged
  (params (Health :type Float%20%28single-precision%29) (MaxHealth :type Float%20%28single-precision%29))
  (bind _aswbp_hud (Utilities|Casting|CastToWBP_HUD (Variables|Default|GetDefaultHUDWidget)))
  (Default|SetHealthBarPercent _aswbp_hud (/ Health MaxHealth)))

(event EventOnCyberdeckRAMChanged
  (params (CyberdeckRAM :type Float%20%28single-precision%29) (MaxCyberdeckRAM :type Float%20%28single-precision%29) (Ratio :type Float%20%28single-precision%29))
  (bind _aswbp_quick_hack_hud (Utilities|Casting|CastToWBP_QuickHackHUD (Variables|Default|GetQuickHackWidget)))
  (Default|UpdateRAMValueText _aswbp_quick_hack_hud (Utilities|Text|FormatText "{RAM} / {MaxRAM}" CyberdeckRAM MaxCyberdeckRAM))
  (Variables|/Game/MyGame/Blueprints/UI/WBP_QuickHackHUD.WBP_QuickHackHUD_C|SetMaxRAM _aswbp_quick_hack_hud (Math|Float|Truncate MaxCyberdeckRAM))
  (Variables|/Game/MyGame/Blueprints/UI/WBP_QuickHackHUD.WBP_QuickHackHUD_C|SetCurrentRAM _aswbp_quick_hack_hud (Math|Float|Truncate CyberdeckRAM))
  (Default|AddRAMtoRAMHorizontalBox _aswbp_quick_hack_hud))

(event EventTick
  (params (DeltaSeconds :type Float%20%28single-precision%29))
  (if (Variables|Default|GetbStartLineTrace)
    (CallFunction|DoLineTrace)
    (else
      (Variables|Default|SetbTargetAquired false)
      (Variables|Default|SetQuickHackTarget 0))))

(event EventSetDefaultUIValues
  (bind _attributes (Variables|Default|GetAttributes))
  (bind _attributes_2 (Variables|Default|GetAttributes))
  (bind _cyberdeckram (Variables|/Script/QuickHack.GenericAttributeSet|GetCyberdeckRAM _attributes))
  (bind _maxcyberdeckram (Variables|/Script/QuickHack.GenericAttributeSet|GetMaxCyberdeckRAM _attributes))
  (bind _currentvalue (Utilities|Struct|BreakGameplayAttributeData _maxcyberdeckram))
  (bind _currentvalue_2 (Utilities|Struct|BreakGameplayAttributeData _cyberdeckram))
  (bind _aswbp_hud (Utilities|Casting|CastToWBP_HUD (Variables|Default|GetDefaultHUDWidget)))
  (Default|SetHealthBarPercent _aswbp_hud (/ (.CurrentValue (Utilities|Struct|BreakGameplayAttributeData (Variables|/Script/QuickHack.GenericAttributeSet|GetHealth _attributes_2))) (.CurrentValue (Utilities|Struct|BreakGameplayAttributeData (Variables|/Script/QuickHack.GenericAttributeSet|GetMaxHealth _attributes_2)))))
  (bind _aswbp_quick_hack_hud (Utilities|Casting|CastToWBP_QuickHackHUD (Variables|Default|GetQuickHackWidget)))
  (Default|UpdateRAMValueText _aswbp_quick_hack_hud (Utilities|Text|FormatText "{RAM} / {MaxRAM}" _currentvalue_2 _currentvalue))
  (Variables|/Game/MyGame/Blueprints/UI/WBP_QuickHackHUD.WBP_QuickHackHUD_C|SetMaxRAM _aswbp_quick_hack_hud (Math|Float|Truncate _currentvalue))
  (Variables|/Game/MyGame/Blueprints/UI/WBP_QuickHackHUD.WBP_QuickHackHUD_C|SetCurrentRAM _aswbp_quick_hack_hud (Math|Float|Truncate _currentvalue_2))
  (Default|AddRAMtoRAMHorizontalBox _aswbp_quick_hack_hud))

(event EventBeginPlay
  (Variables|Default|SetQuickHackPanelCount 0)
  (bind _output_get (Variables|Default|SetCurrentSelectedPanelIndex 0))
  (bind _aswbp_quick_hack_hud (Utilities|Casting|CastToWBP_QuickHackHUD (Variables|Default|GetQuickHackWidget)))
  (Default|SetSelectedQuickHackPanel _aswbp_quick_hack_hud _output_get)
  (Default|CallOnQuickHackTargetAquired false)
  (Variables|Default|SetCounterTest 0)
  (bind _index (Utilities|FlowControl|ForLoopwithBreak 0 5)
    (:LoopBody
      (Development|PrintString (Utilities|String|ToString(Integer) (- (+ _index 5) (Variables|Default|GetCounterTest))))
      (Variables|Default|SetCounterTest (+ (Variables|Default|GetCounterTest) 2)))))

(event Input|ActionEvents|InputActionListMoveUp
  (params (Key :type Key%20Structure :default "None"))
  ;[1 1 1] QuickHack Panel UI Selection
  (:Pressed
    (bind _output_get (Variables|Default|SetCurrentSelectedPanelIndex (+ (Variables|Default|GetCurrentSelectedPanelIndex) -1)))
    (if (< _output_get 0)
      (Variables|Default|SetCurrentSelectedPanelIndex (- (Variables|Default|GetQuickHackPanelCount) 1)))
    (bind _aswbp_quick_hack_hud (Utilities|Casting|CastToWBP_QuickHackHUD (Variables|Default|GetQuickHackWidget)))
    (Default|SetSelectedQuickHackPanel _aswbp_quick_hack_hud (Variables|Default|GetCurrentSelectedPanelIndex))))

(event Input|ActionEvents|InputActionListMoveDown
  (params (Key :type Key%20Structure :default "None"))
  ;[1 1 1] QuickHack Panel UI Selection
  (:Pressed
    (bind _output_get (Variables|Default|SetCurrentSelectedPanelIndex (+ (Variables|Default|GetCurrentSelectedPanelIndex) 1)))
    (if (> _output_get (- (Variables|Default|GetQuickHackPanelCount) 1))
      (Variables|Default|SetCurrentSelectedPanelIndex 0))
    (bind _aswbp_quick_hack_hud (Utilities|Casting|CastToWBP_QuickHackHUD (Variables|Default|GetQuickHackWidget)))
    (Default|SetSelectedQuickHackPanel _aswbp_quick_hack_hud (Variables|Default|GetCurrentSelectedPanelIndex))))

(event Input|ActionEvents|InputActionQuickHackConfirm
  (params (Key :type Key%20Structure :default "None"))
  ;[1 1 1] Executing the selected UI
  (:Pressed
    (bind _aswbp_quick_hack_hud (Utilities|Casting|CastToWBP_QuickHackHUD (Variables|Default|GetQuickHackWidget)))
    (bind (_abilityclass _ability_tag) (Default|GetAbilityTagandClassbySelectedIndex _aswbp_quick_hack_hud (Variables|Default|GetCurrentSelectedPanelIndex)))
    (CallFunction|PerformQuickHack _ability_tag (.Value (Utilities|Map|Find (Variables|Default|GetAbilityInfosMap) _abilityclass)) _abilityclass)
    (Default|SetSelectedQuickHackPanel _aswbp_quick_hack_hud (Variables|Default|GetCurrentSelectedPanelIndex))))

(fn ConstructionScript)