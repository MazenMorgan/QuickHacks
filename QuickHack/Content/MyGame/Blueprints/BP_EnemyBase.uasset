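; BP_EnemyBase is a base enemy Blueprint that shows health and receives quickhack uploads through widget components.
; The health bar initializes from current and max Health attributes and refreshes on health changes.
; Starting an upload feeds the quickhack info to the upload bar and flags the enemy, while gain or loss of the QH.Uploading gameplay tag toggles blocking of all quickhacks.
; Death hides both bars.
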(event Custom|StartQuickHackUpload
  (params (QuickHackInfo :type Gameplay%20Quick%20Hack%20Ability%20Info%20Structure))
  (bind _aswbp_upload_bar (Utilities|Casting|CastToWBP_UploadBar (UserInterface|GetUserWidgetObject (Variables|Default|GetUploadBarWidget))))
  (Default|SetQuickHackInfos _aswbp_upload_bar QuickHackInfo)
  (Default|DoUpload _aswbp_upload_bar)
  (Variables|Default|SetbIsQHUploadingOnSelf true))

(event Custom|OnTagAquiredOrRemovedEvent
  (params (bTagAquired :type Boolean) (GameplayTag :type Gameplay%20Tag%20Structure))
  (bind _returnvalue (== GameplayTag "(TagName=\"QH.Uploading\")"))
  (if bTagAquired
    (if _returnvalue
      (Variables|Default|SetbBlockAllQuickHacks true))
    (elif _returnvalue
      (Variables|Default|SetbBlockAllQuickHacks false))))

(event EventBeginPlay
  (bind _attributes (Variables|Default|GetAttributes))
  (EventDispatchers|BindEventtoOnTagAquiredorRemoved (delegate Custom|OnTagAquiredOrRemovedEvent))
  (bind _aswbp_health_bar (Utilities|Casting|CastToWBP_HealthBar (UserInterface|GetUserWidgetObject (Variables|Default|GetHealthBarWidget))))
  (Default|SetHealthbarProgressasPercentage _aswbp_health_bar (/ (.CurrentValue (Utilities|Struct|BreakGameplayAttributeData (Variables|/Script/QuickHack.GenericAttributeSet|GetHealth _attributes))) (.CurrentValue (Utilities|Struct|BreakGameplayAttributeData (Variables|/Script/QuickHack.GenericAttributeSet|GetMaxHealth _attributes))))))

(event EventDie
  (Rendering|SetVisibility (Variables|Default|GetHealthBarWidget) false false)
  (Rendering|SetVisibility (Variables|Default|GetUploadBarWidget) false false))

(event EventOnHealthChanged
  (params (Health :type Float%20%28single-precision%29) (MaxHealth :type Float%20%28single-precision%29))
  (bind _aswbp_health_bar (Utilities|Casting|CastToWBP_HealthBar (UserInterface|GetUserWidgetObject (Variables|Default|GetHealthBarWidget))))
  (Default|SetHealthbarProgressasPercentage _aswbp_health_bar (/ Health MaxHealth)))

(fn ConstructionScript)